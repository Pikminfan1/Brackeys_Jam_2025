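; Game mode that tracks live race positions for registered karts.
; AddKart registers each kart in a progress map, and a looping timer started on BeginPlay refreshes every kart's course progress several times a second.
; Each refresh ranks karts from most to least progress by repeatedly extracting the maximum from parallel arrays, then broadcasts the ordered list through the OnPositionUpdate dispatcher.
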(event `self.ReceiveBeginPlay`
  (`KismetSystemLibrary.K2_SetTimer` null "GetKartProgress" 0.2 true))

(fn `AddKart`
  (params (Kart :type "/Game/Blueprints/BP_Kart Object Reference"))
  (`BlueprintMapLibrary.Map_Add` (`self.KartProgress`) Kart))

(fn `GetKartProgress`
  (locals (UnsortedProgress :type "Array of Float (double-precision)") (UnsortedKarts :type "Array of /Game/Blueprints/BP_Kart Object Reference"))
  (bind _kartprogress (`self.KartProgress`))
  (bind _indexofmaxvalue (`KismetMathLibrary.MaxOfFloatArray` (`local.UnsortedProgress`)))
  (`KismetArrayLibrary.Array_Clear` (`self.KartPositions`))
  (bind _keys (`BlueprintMapLibrary.Map_Keys` (`self.KartProgress`)))
  (for _array_element _keys
    (`BlueprintMapLibrary.Map_Add` (`self.KartProgress`) _array_element (`/Game/Blueprints/BP_Kart.GetCourseProgress` _array_element)))
  (bind _values (`BlueprintMapLibrary.Map_Values` _kartprogress))
  (bind _output_get (set `local.UnsortedProgress` _values))
  (bind _keys_2 (`BlueprintMapLibrary.Map_Keys` _kartprogress))
  (set `local.UnsortedKarts` _keys_2)
  (while (> (`KismetArrayLibrary.Array_Length` _output_get) 0)
    (`KismetArrayLibrary.Array_Add` (`self.KartPositions`) (`|GetArrayItem` (`local.UnsortedKarts`) _indexofmaxvalue))
    (`KismetArrayLibrary.Array_Remove` (`local.UnsortedKarts`) _indexofmaxvalue)
    (`KismetArrayLibrary.Array_Remove` (`local.UnsortedProgress`) _indexofmaxvalue))
  (`self.OnPositionUpdate` (`self.KartPositions`)))

(fn `UserConstructionScript`)