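; BP_Bomb is a bomb hazard that kills any living kart pawn that overlaps it.
; On overlap it sets both the kart and itself dead through SetIsDead.
; HandleOnDeath, apparently bound at BeginPlay to the killable actor's IsDead change event, hides the mesh and disables sphere collision on death, restoring both when revived.
; The handler also prints the new state to screen.
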(event `self.ReceiveBeginPlay`
  (add `self.OnIsDeadChangedKillableActor` (`|CreateDelegate` :!event `HandleOnDeath`)))

(event `self.ReceiveActorBeginOverlap`
  (params (OtherActor :type "Actor Object Reference"))
  (bind _askart_pawn_base (cast `KartPawnBase` OtherActor))
  (if (not (`KartPawnBase.bIsDead` _askart_pawn_base))
    (`KartPawnBase.SetIsDead` _askart_pawn_base true)
    (`Killable.SetIsDead` true)))

(event `HandleOnDeath` :!signature `self.OnIsDeadChangedKillableActor`
  (params (bNewIsDead :type Boolean))
  (`KismetSystemLibrary.PrintString` (`KismetStringLibrary.Conv_BoolToString` bNewIsDead))
  (if bNewIsDead
    (`SceneComponent.SetVisibility` (`self.SkeletalMesh`) false false)
    (`PrimitiveComponent.SetCollisionEnabled` (`self.Sphere`) "NoCollision")
    (else
      (`SceneComponent.SetVisibility` (`self.SkeletalMesh`) true false)
      (`PrimitiveComponent.SetCollisionEnabled` (`self.Sphere`) "QueryAndPhysics"))))

(fn `UserConstructionScript`)