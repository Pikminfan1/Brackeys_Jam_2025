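; Laser gate field hazard that kills any living kart pawn that begins overlapping it.
; A looping timer toggles Active through a FlipFlop, and Tick interpolates the actor's scale toward zero while Active, or back to full size otherwise, with Z snapping back instantly.
; Rewind component events pause the timer during time manipulation and resume it afterward, without adjusting for the rewound time.
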(event `self.ReceiveActorBeginOverlap`
  (params (OtherActor :type "Actor Object Reference"))
  (bind _askart_pawn_base (cast `KartPawnBase` OtherActor))
  (if (not (`KartPawnBase.bIsDead` _askart_pawn_base))
    (`KartPawnBase.SetIsDead` _askart_pawn_base true)))

(event `self.ReceiveBeginPlay`
  (bind _rewind (`self.Rewind`))
  (bind _returnvalue (`KismetSystemLibrary.K2_SetTimerDelegate` (`|CreateDelegate` :!event `TimerEvent`) (`self.Time To activate Field`) true))
  (set `self.Timer Handle` _returnvalue)
  (add `RewindComponent.OnTimeManipulationStarted` _rewind (`|CreateDelegate` :!event `HandleTimePause`))
  (add `RewindComponent.OnTimeManipulationCompleted` _rewind (`|CreateDelegate` :!event `HandleTimeResume`)))

(event `self.ReceiveTick`
  (params (DeltaSeconds :type "Float (single-precision)"))
  (bind (_returnvalue_x _returnvalue_y _returnvalue_z) (`KismetMathLibrary.BreakVector` (`self.GetActorScale3D`)))
  (bind (_returnvalue_x_2 _returnvalue_y_2 _returnvalue_z_2) (`KismetMathLibrary.BreakVector` (`self.GetActorScale3D`)))
  (bind _interp_speed (`self.Interp Speed`))
  (bind _interp_speed_2 (`self.Interp Speed`))
  (if (`self.Active`)
    (`self.SetActorScale3D` (`KismetMathLibrary.MakeVector` (`KismetMathLibrary.FInterpTo` _returnvalue_x 0.0 DeltaSeconds _interp_speed) (`KismetMathLibrary.FInterpTo` _returnvalue_y 0.0 DeltaSeconds _interp_speed) (`KismetMathLibrary.FInterpTo` _returnvalue_z 0.0 DeltaSeconds 1.0)))
    (else
      (`self.SetActorScale3D` (`KismetMathLibrary.MakeVector` (`KismetMathLibrary.FInterpTo` _returnvalue_x_2 1.0 DeltaSeconds _interp_speed_2) (`KismetMathLibrary.FInterpTo` _returnvalue_y_2 1.0 DeltaSeconds _interp_speed_2) 1.0)))))

(event `TimerEvent`
  (bind _isa (`/Engine/EditorBlueprintResources/StandardMacros.FlipFlop`)
    (:`A`
      (set `self.Active` _isa))
    (:`B`
      (set `self.Active` _isa))))

(event `HandleTimePause`
  (`KismetSystemLibrary.K2_PauseTimerHandle` (`self.Timer Handle`)))

(event `HandleTimeResume`
  (params (TotalRewindTime :type "Float (single-precision)"))
  (`KismetSystemLibrary.K2_UnPauseTimerHandle` (`self.Timer Handle`)))

(fn `UserConstructionScript`)