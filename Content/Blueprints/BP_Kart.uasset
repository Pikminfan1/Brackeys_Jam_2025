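; Physics-driven racing kart pawn, driven by player input or spline-following AI, with time pause, rewind and fast-forward through RewindGameMode.
; Each Tick, four wheel raycasts apply suspension and drive forces to the chassis box, with torque for steering and a boost on drift start.
; The track spline supplies AI steering and throttle, course progress and a timed reset when toppled.
; Death freezes physics and swaps material, and the player's rewound time feeds the game mode timer.
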(event `EnhancedInput|/Game/Inputs/IA_Rewind`
  (params (ActionValue :type Boolean) (ElapsedSeconds :type "Float (double-precision)") (TriggeredSeconds :type "Float (double-precision)") (InputAction :type "InputAction Object Reference" :default "/Game/Inputs/IA_Rewind.IA_Rewind"))
  (bind _rewind_game_mode (`self.Rewind Game Mode`))
  ; Rewind Events
  (:`Started`
    (if (`self.IsTimePaused`)
      (`RewindGameMode.StartGlobalRewind` _rewind_game_mode)))
  (:`Completed`
    (if (`self.IsTimePaused`)
      (`RewindGameMode.StopGlobalRewind` _rewind_game_mode))))

(event `OnTimeManipulationCompleted_Event`
  (params (TotalRewindTime :type "Float (single-precision)"))
  ; Initialize Required Kart Components and Player UI
  ;; Clean this, but this will report on things that need to occur during time scrub and on finishing, reporting the time spent rewound
  (if (== (`self.GetController`) (`GameplayStatics.GetPlayerController` 0))
    (`RewindComponent.ResetTotalRewindTime` (`self.Rewind`))
    (`/Game/Blueprints/BP_TestGamemode.ReduceTime` (`self.As BP Test Gamemode`) TotalRewindTime)
    (set `/Game/Blueprints/BP_TestGamemode.bIsTimeStopped` false (`self.As BP Test Gamemode`))))

(event `self.ReceiveBeginPlay`
  ; Initialize Required Kart Components and Player UI
  (set `self.StartingMaterial` (`PrimitiveComponent.GetMaterial` (`self.Cube`) 0))
  (set `self.Name` (`KismetSystemLibrary.GetObjectName` self))
  (`EnhancedInputSubsystemInterface.AddMappingContext` (pcsubsystem `EnhancedInputLocalPlayerSubsystem` (`GameplayStatics.GetPlayerController` 0)) "/Game/Inputs/IMC_Vehicle.IMC_Vehicle" 0 (struct))
  (bind _returnvalue (`GameplayStatics.GetActorOfClass` "/Game/Blueprints/BP_TrackSpline.BP_TrackSpline_C"))
  (`/Engine/EditorBlueprintResources/StandardMacros.IsValid` _returnvalue
    (:`Is Valid`
      (set `self.Track` _returnvalue)
      (bind _returnvalue_2 (`|CreateWidget` "/Game/UI/WBP_HUD.WBP_HUD_C"))
      (`/Engine/EditorBlueprintResources/StandardMacros.IsValid` _returnvalue_2
        (:`Is Valid`
          ;; I Don't think I need both of these
          (`UserWidget.AddToViewport` _returnvalue_2 0)
          (`UserWidget.AddToPlayerScreen` _returnvalue_2 0)
          (bind _asbp_test_gamemode (cast `/Game/Blueprints/BP_TestGamemode` (`GameplayStatics.GetGameMode`)))
          (`/Game/Blueprints/BP_TestGamemode.AddKart` _asbp_test_gamemode self)
          (bind _asrewind_game_mode (cast `RewindGameMode` (`GameplayStatics.GetGameMode`)))
          (`/Engine/EditorBlueprintResources/StandardMacros.IsValid` _asrewind_game_mode
            (:`Is Valid`
              (bind _output_get (set `self.Rewind Game Mode` _asrewind_game_mode))
              ;; Clean this, but this will report on things that need to occur during time scrub and on finishing, reporting the time spent rewound
              (add `self.OnIsDeadChanged` (`|CreateDelegate` :!event `HandleOnIsDead`))
              (add `RewindGameMode.OnGlobalTimeScrubStarted` _output_get (`|CreateDelegate` :!event `HandleOnTimeScrubStarted`))
              (add `RewindGameMode.OnGlobalTimeScrubCompleted` _output_get (`|CreateDelegate` :!event `HandleOnTimeScrubComplete`))
              (add `RewindComponent.OnTimeManipulationCompleted` (`self.Rewind`) (delegate `OnTimeManipulationCompleted_Event`))
              ; I am ashamed of this
              (bind _asbp_test_gamemode_2 (cast `/Game/Blueprints/BP_TestGamemode` (`self.Rewind Game Mode`)))
              (set `self.As BP Test Gamemode` _asbp_test_gamemode_2))))))
    (:`Is Not Valid`
      (`KismetSystemLibrary.PrintString` "No Track Spline found in Level" true true (struct :`R` 1.0 :`B` 0.070897 :`A` 1.0)))))

(event `EnhancedInput|/Game/Inputs/IA_FastForward`
  (params (ActionValue :type Boolean) (ElapsedSeconds :type "Float (double-precision)") (TriggeredSeconds :type "Float (double-precision)") (InputAction :type "InputAction Object Reference" :default "/Game/Inputs/IA_FastForward.IA_FastForward"))
  (bind _rewind_game_mode (`self.Rewind Game Mode`))
  ; Rewind Events
  (:`Started`
    (if (`self.IsTimePaused`)
      (`RewindGameMode.StartGlobalFastForward` _rewind_game_mode)))
  (:`Completed`
    (if (`self.IsTimePaused`)
      (`RewindGameMode.StopGlobalFastForward` _rewind_game_mode))))

(event `EnhancedInput|/Game/Inputs/IA_PauseTime`
  (params (ActionValue :type Boolean) (ElapsedSeconds :type "Float (double-precision)") (TriggeredSeconds :type "Float (double-precision)") (InputAction :type "InputAction Object Reference" :default "/Game/Inputs/IA_PauseTime.IA_PauseTime"))
  ; Rewind Events
  (:`Started`
    (`RewindGameMode.ToggleTimeScrub` (`self.Rewind Game Mode`))))

(event `self.ReceiveAsyncPhysicsTick`
  (params (DeltaSeconds :type "Float (single-precision)") (SimSeconds :type "Float (single-precision)"))
  ; Apply Physics Forces on Suspension, and acceleration on the chasis, Should prolly move to async physics but I'm too afraid rn
)

(event `self.ReceiveTick`
  (params (DeltaSeconds :type "Float (single-precision)"))
  ; Apply Physics Forces on Suspension, and acceleration on the chasis, Should prolly move to async physics but I'm too afraid rn
  (if (not (or (`self.IsTimePaused`) (`self.bIsDead`)))
    (`|ExecutionSequence`
      (:`then_0`
        (`|ExecutionSequence`
          (:`then_0`
            (bind _groundcheck (`self.SuspensionRaycast` (`self.FL_Wheel`))))
          (:`then_1`
            (bind _groundcheck_2 (`self.SuspensionRaycast` (`self.FR_Wheel`))))
          (:`then_2`
            (bind _groundcheck_3 (`self.SuspensionRaycast` (`self.BR_Wheel`))))
          (:`then_3`
            (bind _groundcheck_4 (`self.SuspensionRaycast` (`self.BL_Wheel`)))
            (if (and _groundcheck _groundcheck_2 _groundcheck_3 _groundcheck_4)
              (`KismetSystemLibrary.K2_ClearAndInvalidateTimerHandle` (`self.ResetTimer_Handle`))))
          (:`then_4`
            (`self.CalculateAcceleration`)
            ;[0.15 0 0.004199 0.5] Disconect This node to prevent reorientation
            (`self.IsToppled`))
          (:`then_5`
            (if (`self.bIsDead`)
              _))
          (:`then_6`
            ; MPH
            (if (== (`self.GetController`) (`GameplayStatics.GetPlayerController` 0))
              (`KismetSystemLibrary.PrintString` (`KismetTextLibrary.Conv_TextToString` (`|FormatText` "{kph} KM/H" (/ (`KismetMathLibrary.FFloor` (* (* (`KismetMathLibrary.VSize` (`self.GetVelocity`)) 0.036) 10.0)) 10))) true true (struct :`R` 1.0 :`G` 0.039222 :`A` 1.0) 0.0)))))
      (:`then_1`
        ;; AI Driving Logic
        (if (!= (`self.GetController`) (`GameplayStatics.GetPlayerController` 0))
          (`self.AI_AccelerateKart` (`self.GetAIThrottle`))
          (`self.AI_SteerKart` (`self.GetAISteering`)))))))

(event `HandleOnTimeScrubStarted`
  ; Handle When Rewind Scrub Begins
  (set `self.IsTimePaused` true)
  (set `/Game/Blueprints/BP_TestGamemode.bIsTimeStopped` true (`self.As BP Test Gamemode`)))

(event `HandleOnTimeScrubComplete`
  ; Handle When Rewind Scrub Begins
  (set `self.IsTimePaused` false))

(event `EnhancedInput|/Game/Inputs/IA_HandBrake`
  (params (ActionValue :type Boolean) (ElapsedSeconds :type "Float (double-precision)") (TriggeredSeconds :type "Float (double-precision)") (InputAction :type "InputAction Object Reference" :default "/Game/Inputs/IA_HandBrake.IA_HandBrake"))
  (:`Triggered`
    (set `self.IsHandBraking` ActionValue :!label _label)
    (if (not (or (`self.IsTimePaused`) (`self.bIsDead`)))
      (set `self.AccelerationInput` (`KismetMathLibrary.FInterpTo` (`self.AccelerationInput`) (`KismetMathLibrary.SelectFloat` 0.0 0.0 (`self.IsOnGround`)) (`GameplayStatics.GetWorldDeltaSeconds`) (`self.HandBrakeScalar`)))))
  (:`Ongoing`
    (goto _label))
  (:`Canceled`
    (set `self.IsHandBraking` false :!label _label_2))
  (:`Completed`
    (goto _label_2)))

(event `EnhancedInput|/Game/Inputs/IA_Accelerate`
  (params (ActionValue :type "Float (double-precision)") (ElapsedSeconds :type "Float (double-precision)") (TriggeredSeconds :type "Float (double-precision)") (InputAction :type "InputAction Object Reference" :default "/Game/Inputs/IA_Accelerate.IA_Accelerate"))
  ; Interpolate towards our desired acceleration unless we are in the air
  (:`Triggered`
    (if (`self.IsHandBraking`)
      _
      (elif (not (or (`self.IsTimePaused`) (`self.bIsDead`)))
        (set `self.AccelerationInput` (`KismetMathLibrary.FInterpTo` (`self.AccelerationInput`) (`KismetMathLibrary.SelectFloat` ActionValue 0.0 (`self.IsOnGround`)) (`GameplayStatics.GetWorldDeltaSeconds`) 0.5))))))

(event `EnhancedInput|/Game/Inputs/IA_Drift`
  (params (ActionValue :type Boolean) (ElapsedSeconds :type "Float (double-precision)") (TriggeredSeconds :type "Float (double-precision)") (InputAction :type "InputAction Object Reference" :default "/Game/Inputs/IA_Drift.IA_Drift"))
  ; Drift Mechanic
  (:`Started`
    (if (not (or (`self.IsTimePaused`) (`self.bIsDead`)))
      (`self.StartDrift`)))
  (:`Canceled`
    (if (not (or (`self.IsTimePaused`) (`self.bIsDead`))) :!label _label_3
      (`self.StopDrift`)))
  (:`Completed`
    (goto _label_3)))

(event `EnhancedInput|/Game/Inputs/IA_Steer`
  (params (ActionValue :type "Float (double-precision)") (ElapsedSeconds :type "Float (double-precision)") (TriggeredSeconds :type "Float (double-precision)") (InputAction :type "InputAction Object Reference" :default "/Game/Inputs/IA_Steer.IA_Steer"))
  (bind (_driftrotation_roll _driftrotation_pitch _driftrotation_yaw) (`KismetMathLibrary.BreakRotator` (`self.DriftRotation`)))
  (bind (_relativerotation_roll _relativerotation_pitch _relativerotation_yaw) (`KismetMathLibrary.BreakRotator` (`SceneComponent.RelativeRotation` (`self.FL_Wheel`))))
  ; Apply Rotation to the wheels, add torque to the chasis to steer
  (:`Triggered`
    (if (not (or (`self.IsTimePaused`) (`self.bIsDead`)))
      (set `self.DriftSteer` (`KismetMathLibrary.FClamp` (`KismetMathLibrary.SelectFloat` (* (`KismetMathLibrary.FMax` (`self.DriftSteer`) (`KismetMathLibrary.Abs` ActionValue)) (`KismetMathLibrary.SignOfFloat` _driftrotation_yaw)) ActionValue (`self.IsDrifting`)) -3.0 3.0))
      (`PrimitiveComponent.AddTorqueInRadians` (`self.Box`) (`KismetMathLibrary.MakeVector` 0.0 0.0 (* ActionValue (`self.SteeringTorque`) (* (`self.AccelerationInput`) (`self.SteerlingMultiplier`)))) "None" false)
      (`SceneComponent.K2_SetRelativeRotation` (`self.FL_Wheel`) (`KismetMathLibrary.MakeRotator` 0.0 0.0 (`KismetMathLibrary.FInterpTo` _relativerotation_yaw (`|GetInputActionValue`) (`GameplayStatics.GetWorldDeltaSeconds`) 3.0)) false false)
      (`SceneComponent.K2_SetRelativeRotation` (`self.FR_Wheel`) (`KismetMathLibrary.MakeRotator` 0.0 0.0 (`KismetMathLibrary.FInterpTo` _relativerotation_yaw (`|GetInputActionValue`) (`GameplayStatics.GetWorldDeltaSeconds`) 3.0)) false false))))

(event `HandleOnIsDead` :!signature `self.OnIsDeadChanged`
  (params (bNewIsDead :type Boolean))
  (bind _box (`self.Box`))
  (if (not bNewIsDead)
    (if (`RewindGameMode.IsGlobalRewinding` (`self.Rewind Game Mode`))
      ; Kart Comes Back to Life
      (`PrimitiveComponent.SetMaterial` (`self.Cube`) 0 (`self.StartingMaterial`))
      (`ActorComponent.SetActive` (`self.NS_DeathFX`) false false)
      (`KismetSystemLibrary.PrintString` (`KismetStringLibrary.Concat_StrStr` (`self.Name`) " is alive!") true true (struct :`R` 0.85625 :`G` 0.099273 :`B` 0.68146 :`A` 1.0))
      (`PrimitiveComponent.SetSimulatePhysics` (`self.Box`) true)
      (else
        ; Kart Dies
        (`PrimitiveComponent.SetMaterial` (`self.Cube`) 0 "/Engine/EditorMaterials/GridMaterial.GridMaterial" :!label _label_4)
        (`ActorComponent.SetActive` (`self.NS_DeathFX`) true false)
        (`KismetSystemLibrary.PrintString` (`KismetStringLibrary.Concat_StrStr` (`self.Name`) " is dead"))
        (`PrimitiveComponent.SetAllPhysicsLinearVelocity` _box (0.0 0.0 0.0) false)
        (`PrimitiveComponent.SetAllPhysicsAngularVelocityInRadians` _box (0.0 0.0 0.0) false)
        (`PrimitiveComponent.SetSimulatePhysics` _box false)))
    (else
      (goto _label_4))))

(fn `AccelerateKart`
  (params (WheelComp :type "SceneComponent Object Reference") (ImpactNormal :type "Vector Structure"))
  (bind _box (`self.Box`))
  (`PrimitiveComponent.AddForceAtLocation` (`self.Box`) (+ (* (`SceneComponent.GetForwardVector` _box) (`self.TopSpeed`) (`self.AccelerationInput`) (`PrimitiveComponent.GetMass` _box) (`self.SpeedModifier`)) (`KismetMathLibrary.SelectVector` (0.0 0.0 0.0) (`KismetMathLibrary.MakeVector` 0.0 0.0 (`self.DownForceInAir`)) (`self.IsOnGround`))) (`SceneComponent.K2_GetComponentLocation` WheelComp) "None"))

(fn `AI_AccelerateKart`
  (params (Throttle :type "Float (double-precision)"))
  ; Interpolate towards our desired acceleration unless we are in the air
  (set `self.AccelerationInput` (`KismetMathLibrary.FInterpTo` (`self.AccelerationInput`) (`KismetMathLibrary.SelectFloat` Throttle (`self.AccelerationInput`) (`self.IsOnGround`)) (`GameplayStatics.GetWorldDeltaSeconds`) 0.5)))

(fn `AI_SteerKart`
  (params (SteerDirection :type "Float (double-precision)"))
  (bind (_relativerotation_roll _relativerotation_pitch _relativerotation_yaw) (`KismetMathLibrary.BreakRotator` (`SceneComponent.RelativeRotation` (`self.FL_Wheel`))))
  ; Apply Rotation to the wheels, add torque to the chasis to steer
  (`PrimitiveComponent.AddTorqueInRadians` (`self.Box`) (`KismetMathLibrary.MakeVector` 0.0 0.0 (* SteerDirection (`self.SteeringTorque`) (`self.AccelerationInput`) (`self.SteerlingMultiplier`))) "None" false)
  (`SceneComponent.K2_SetRelativeRotation` (`self.FL_Wheel`) (`KismetMathLibrary.MakeRotator` 0.0 0.0 (`KismetMathLibrary.FInterpTo` _relativerotation_yaw SteerDirection (`GameplayStatics.GetWorldDeltaSeconds`) 3.0)) false false)
  (`SceneComponent.K2_SetRelativeRotation` (`self.FR_Wheel`) (`KismetMathLibrary.MakeRotator` 0.0 0.0 (`KismetMathLibrary.FInterpTo` _relativerotation_yaw SteerDirection (`GameplayStatics.GetWorldDeltaSeconds`) 3.0)) false false))

(fn `BoostKart`
  (params (SpeedModifier :type "Float (double-precision)") (Time :type "Float (double-precision)"))
  (if (`KismetSystemLibrary.K2_IsTimerActiveHandle` (`self.BoostTimer_Handle`))
    (`KismetSystemLibrary.K2_ClearAndInvalidateTimerHandle` (`self.BoostTimer_Handle`)))
  (set `self.SpeedModifier` SpeedModifier)
  (bind _returnvalue (`KismetSystemLibrary.K2_SetTimer` null "ResetSpeed" Time))
  (set `self.BoostTimer_Handle` _returnvalue))

(fn `CalculateAcceleration`
  (bind _output_get (set `self.Acceleration` (`KismetMathLibrary.Lerp` 0.0 (`self.MaxAcceleration`) (`self.AccelerationInput`))))
  (bind _output_get_2 (set `self.AccelerationInput` (`KismetMathLibrary.FInterpTo` (`self.AccelerationInput`) 0.0 (`GameplayStatics.GetWorldDeltaSeconds`) 0.3)))
  (`SceneComponent.K2_AddLocalRotation` (`self.Wheel_BL`) (`KismetMathLibrary.MakeRotator` 0.0 (/ _output_get -1000.0)) false false)
  (`SceneComponent.K2_AddLocalRotation` (`self.Wheel_BR`) (`KismetMathLibrary.MakeRotator` 0.0 (/ _output_get -1000.0)) false false)
  (`SceneComponent.K2_AddLocalRotation` (`self.Wheel_FR`) (`KismetMathLibrary.MakeRotator` 0.0 (/ _output_get -1000.0)) false false)
  (`SceneComponent.K2_AddLocalRotation` (`self.Wheel_FL`) (`KismetMathLibrary.MakeRotator` 0.0 (/ _output_get -1000.0)) false false)
  (`SceneComponent.K2_SetRelativeRotation` (`self.Pivot`) (`KismetMathLibrary.RInterpTo` (`SceneComponent.RelativeRotation` (`self.Pivot`)) (`self.DriftRotation`) (`GameplayStatics.GetWorldDeltaSeconds`) 3.0) false false))

(fn `GetAISteering`
  (returns (ReturnValue :type "Float (double-precision)"))
  (bind _returnvalue (`KismetMathLibrary.Dot_VectorVector` (`SplineComponent.FindDirectionClosestToWorldLocation` (`/Game/Blueprints/BP_TrackSpline.Spline` (`self.Track`)) (+ (`self.K2_GetActorLocation`) (* (`self.GetActorForwardVector`) 400.0)) "World") (`self.GetActorRightVector`)))
  (return (* _returnvalue (`self.Acceleration`) (`KismetMathLibrary.MultiplyMultiply_FloatFloat` (+ (`KismetMathLibrary.Abs` _returnvalue) 0.0) 2.0))))

(fn `GetAIThrottle`
  (returns (ReturnValue :type "Float (double-precision)"))
  (bind _returnvalue (`KismetMathLibrary.Dot_VectorVector` (`SplineComponent.FindDirectionClosestToWorldLocation` (`/Game/Blueprints/BP_TrackSpline.Spline` (`self.Track`)) (`self.K2_GetActorLocation`) "World") (`self.GetActorForwardVector`)))
  (return (* (`KismetMathLibrary.FClamp` (`KismetMathLibrary.Abs` _returnvalue) 0.5) (`KismetMathLibrary.SignOfFloat` _returnvalue))))

(fn `GetCourseProgress`
  (returns (ReturnValue :type "Float (double-precision)"))
  (bind _spline (`/Game/Blueprints/BP_TrackSpline.Spline` (`self.Track`)))
  (return (+ (/ (`SplineComponent.GetDistanceAlongSplineAtLocation` _spline (`SplineComponent.FindLocationClosestToWorldLocation` _spline (`self.K2_GetActorLocation`) "World") "World") (`SplineComponent.GetSplineLength` _spline)) (`self.Laps`))))

(fn `GetDriftDirection`
  (bind _returnvalue (`KismetMathLibrary.SignOfFloat` (`|GetInputActionValue`)))
  (if (and (!= _returnvalue 0.0) (`self.IsDrifting`))
    (if (> _returnvalue 0.0)
      (set `self.IsDriftingLeft` false)
      (set `self.IsDriftingRight` true)
      (else
        (set `self.IsDriftingLeft` true)
        (set `self.IsDriftingRight` false)))))

(fn `GetTrackProgress`
  (returns (DistanceAlongTrack :type "Float (double-precision)") (IsCorrectDirection :type Boolean))
  (bind _returnvalue (`self.K2_GetActorLocation`))
  (bind _spline (`/Game/Blueprints/BP_TrackSpline.Spline` (`self.Track`)))
  (bind _returnvalue_2 (> (`KismetMathLibrary.Dot_VectorVector` (`SplineComponent.FindDirectionClosestToWorldLocation` _spline _returnvalue "World") (`KismetMathLibrary.Normal` (`self.GetVelocity`))) 0.0))
  ; Calculate Distance along Track Spline and Return the value along with  if we are facing the right direction
  (`KismetSystemLibrary.PrintString` (`KismetMathLibrary.SelectString` "Correct Direction" "Wrong Direction" _returnvalue_2) true true (struct :`G` 0.66 :`B` 1.0 :`A` 1.0) 0.0)
  (return (`SplineComponent.GetDistanceAlongSplineAtLocation` _spline (`SplineComponent.FindLocationClosestToWorldLocation` _spline _returnvalue "World") "World") _returnvalue_2))

(fn `IsOnGround`
  (returns (ReturnValue :type Boolean))
  (bind _returnvalue (`self.K2_GetActorLocation`))
  (bind (_outhit _returnvalue_2) (`KismetSystemLibrary.LineTraceSingle` _returnvalue (- _returnvalue (0.0 0.0 35.0)) "TraceTypeQuery1"))
  (return _returnvalue_2))

(fn `IsToppled`
  (if (and (< (`KismetMathLibrary.Dot_VectorVector` (`self.GetActorUpVector`) (0.0 0.0 1.0)) 0.8) (not (`KismetSystemLibrary.K2_IsValidTimerHandle` (`self.ResetTimer_Handle`))))
    (bind _returnvalue (`KismetSystemLibrary.K2_SetTimerDelegate` (`|CreateDelegate` :!event `ResetPosition`) (`self.TimeUntilKartReorient`)))
    (set `self.ResetTimer_Handle` _returnvalue)))

(fn `ResetPosition`
  (bind _returnvalue (`self.K2_GetActorLocation`))
  (bind _track (`self.Track`))
  (`KismetSystemLibrary.K2_ClearAndInvalidateTimerHandle` (`self.ResetTimer_Handle`))
  (`self.K2_SetActorLocationAndRotation` (`SplineComponent.FindLocationClosestToWorldLocation` (`/Game/Blueprints/BP_TrackSpline.Spline` _track) _returnvalue "World") (`KismetMathLibrary.Conv_VectorToRotator` (`SplineComponent.FindDirectionClosestToWorldLocation` (`/Game/Blueprints/BP_TrackSpline.Spline` _track) _returnvalue "World")))
  (set `self.AccelerationInput` 0.0))

(fn `ResetSpeed`
  (set `self.SpeedModifier` 1.0))

(fn `StartDrift`
  (set `self.SteerlingMultiplier` (`self.DriftSteerMultiplier`))
  (set `self.IsDrifting` true)
  (set `self.DriftRotation` (`KismetMathLibrary.MakeRotator` 0.0 0.0 (* (`KismetMathLibrary.SignOfFloat` (`|GetInputActionValue`)) 25.0)))
  (`self.BoostKart` (+ (/ (`KismetMathLibrary.Abs` (`self.DriftSteer`)) 10.0) 1.0) 1.0))

(fn `StopDrift`
  (set `self.SteerlingMultiplier` 1.0)
  (set `self.IsDrifting` false)
  (set `self.DriftRotation` (struct)))

(fn `SuspensionRaycast`
  (params (`Wheel Comp` :type "SceneComponent Object Reference"))
  (returns (groundCheck :type Boolean))
  (locals (WheelHalfHeight :type "Float (double-precision)" :default 32.0))
  (bind _returnvalue (`SceneComponent.K2_GetComponentLocation` `Wheel Comp`))
  (bind _returnvalue_2 (`SceneComponent.GetChildComponent` (`local.Wheel Comp`) 0))
  (bind (_relativelocation_x _relativelocation_y _relativelocation_z) (`KismetMathLibrary.BreakVector` (`SceneComponent.RelativeLocation` _returnvalue_2)))
  (bind _outhit (`KismetSystemLibrary.LineTraceSingle` :`Start` _returnvalue :`End` (+ _returnvalue (* (`SceneComponent.GetUpVector` `Wheel Comp`) -120.0)) :`TraceChannel` "TraceTypeQuery1" :`DrawDebugType` "ForOneFrame"))
  (bind (_bblockinghit _binitialoverlap _time _distance _location _impactpoint _normal _impactnormal _physmat _hitactor _hitcomponent _hitbonename _bonename _hititem _elementindex _faceindex _tracestart _traceend) (`GameplayStatics.BreakHitResult` _outhit))
  (if _bblockinghit
    (`PrimitiveComponent.AddForceAtLocation` (`self.Box`) (* (- 1.0 (`KismetMathLibrary.NormalizeToRange` _distance 0.0 120.0)) (`KismetMathLibrary.GetDirectionUnitVector` _traceend _tracestart) (`self.SuspensionForceScalar`)) (`SceneComponent.K2_GetComponentLocation` (`local.Wheel Comp`)) "None")
    (`self.AccelerateKart` (`local.Wheel Comp`) _impactnormal)
    (`SceneComponent.K2_SetRelativeLocation` _returnvalue_2 (`KismetMathLibrary.MakeVector` 0.0 0.0 (`KismetMathLibrary.FInterpTo` _relativelocation_z (+ (* _distance -1.0) (`local.WheelHalfHeight`)) (`GameplayStatics.GetWorldDeltaSeconds`) 3.0)) false false)
    (return _bblockinghit)
    (else
      (`self.AccelerateKart` (`local.Wheel Comp`) _impactnormal)
      (return false))))

(fn `UserConstructionScript`
  (bind _returnvalue (`PrimitiveComponent.CreateDynamicMaterialInstance` (`self.Cube`) 0 "/Game/Materials/M_DebugKartMat.M_DebugKartMat" "None"))
  (`MaterialInstanceDynamic.SetVectorParameterValue` _returnvalue "Color" (`self.DebugColor`)))